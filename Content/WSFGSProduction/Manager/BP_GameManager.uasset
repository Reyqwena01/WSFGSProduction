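; Game manager for a crafting game that turns a player's element and tool sequences into crafted results for delivery requests.
; Element and tool picks are resolved by name, with DoOnce gates creating UI tags for certain entries, also reachable through Unlock events.
; After a tool pick, six directions from both are matched against ResultList, notifying the quest UI and playing a sound.
; Delivery creation and failure are stubs; random-order logic is disconnected.
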(event Custom|CreateDelivery
  (params (Difficlity :type Integer))
  (if (not (== Difficlity 0))
    (if (== Difficlity 1)
      _)))

(event Custom|Unlock)

(event Custom|UnlockMetal
  (Utilities|FlowControl|DoOnce false
    (:Completed
      (Default|CreateTag (Variables|/Game/WSFGSProduction/Player/BP_Character.BP_Character_C|GetUi (Variables|Default|GetPlayer)) (Utilities|Array|Get(acopy) (Variables|Default|GetListElement) 2)))))

(event Custom|UnlockCiseau
  (Utilities|FlowControl|DoOnce false
    (:Completed
      (Default|CreateTag (Variables|/Game/WSFGSProduction/Player/BP_Character.BP_Character_C|GetUi (Variables|Default|GetPlayer)) (Utilities|Array|Get(acopy) (Variables|Default|GetListTools) 2)))))

(event Custom|UnlockPonceuse
  (Utilities|FlowControl|DoOnce false
    (:Completed
      (Default|CreateTag (Variables|/Game/WSFGSProduction/Player/BP_Character.BP_Character_C|GetUi (Variables|Default|GetPlayer)) (Utilities|Array|Get(acopy) (Variables|Default|GetListTools) 1)))))

(event Custom|StartTimer
  ;[0.15 0.01906 0.02307 0.5] En fonction de difficulté prend aléatoirement une séquence x fois (quantité en fonction difficulté)
  (bind _result (Math|Float|DecrementFloat (Variables|Default|GetTimer) :!label _label)
    (:%20%20
      (if (<= _result 0.0)
        (CallFunction|DeliveryFail)
        (else
          (Utilities|FlowControl|Delay 1.0)
          (goto _label))))))

(event Custom|DeliveryFail
  ;[0.15 0.01906 0.02307 0.5] En fonction de difficulté prend aléatoirement une séquence x fois (quantité en fonction difficulté)
)

(event Custom|ElementPlayer
  (params (ElementSequence :type S%20Séquence%20Structure))
  (bind _listelement (Variables|Default|GetListElement))
  (bind _listelement_2 (Variables|Default|GetListElement))
  (bind _output (Utilities|Array|Get(acopy) _listelement))
  (bind _output_2 (Utilities|Array|Get(acopy) _listelement_2 2))
  (for _array_element (Variables|Default|GetListElement)
    (if (Utilities|Enum|Equal(Enum) (.Name (Utilities|Struct|BreakS_Séquence _array_element)) (.Name (Utilities|Struct|BreakS_Séquence ElementSequence)))
      (bind _output_get (Variables|Default|SetElementUsed _array_element))
      (Development|PrintString (Utilities|String|ToString(Text) (.name _output_get)))
      (if (Utilities|Enum|Equal(Enum) (.Name (Utilities|Struct|BreakS_Séquence _output)) (.Name (Utilities|Struct|BreakS_Séquence (Variables|Default|GetElementUsed))))
        (Utilities|FlowControl|DoOnce false
          (:Completed
            (Default|CreateTag (Variables|/Game/WSFGSProduction/Player/BP_Character.BP_Character_C|GetUi (Variables|Default|GetPlayer)) _output)))
        (elif (Utilities|Enum|Equal(Enum) (.Name (Utilities|Struct|BreakS_Séquence _output_2)) (.Name (Utilities|Struct|BreakS_Séquence (Variables|Default|GetElementUsed))))
          (Utilities|FlowControl|DoOnce false
            (:Completed
              (Default|CreateTag (Variables|/Game/WSFGSProduction/Player/BP_Character.BP_Character_C|GetUi (Variables|Default|GetPlayer)) _output_2))))))))

(event Custom|ToolPlayer
  (params (ToolSequence :type S%20Séquence%20Structure))
  (bind _listtools (Variables|Default|GetListTools))
  (bind _listtools_2 (Variables|Default|GetListTools))
  (bind _output (Utilities|Array|Get(acopy) _listtools_2 2))
  (bind _output_2 (Utilities|Array|Get(acopy) _listtools 1))
  (for _array_element (Variables|Default|GetListTools)
    (if (Utilities|Enum|Equal(Enum) (.Name (Utilities|Struct|BreakS_Séquence _array_element)) (.Name (Utilities|Struct|BreakS_Séquence ToolSequence)))
      (bind _output_get (Variables|Default|SetToolUsed _array_element))
      (Development|PrintString (Utilities|String|ToString(Text) (.name _output_get)))
      (if (Utilities|Enum|Equal(Enum) (.Name (Utilities|Struct|BreakS_Séquence _output_2)) (.Name (Utilities|Struct|BreakS_Séquence (Variables|Default|GetToolUsed))))
        (Utilities|FlowControl|DoOnce false
          (:Completed
            (Default|CreateTag (Variables|/Game/WSFGSProduction/Player/BP_Character.BP_Character_C|GetUi (Variables|Default|GetPlayer)) _output_2)))
        (elif (Utilities|Enum|Equal(Enum) (.Name (Utilities|Struct|BreakS_Séquence _output)) (.Name (Utilities|Struct|BreakS_Séquence (Variables|Default|GetToolUsed))))
          (Utilities|FlowControl|DoOnce false
            (:Completed
              (Default|CreateTag (Variables|/Game/WSFGSProduction/Player/BP_Character.BP_Character_C|GetUi (Variables|Default|GetPlayer)) _output)))))))
  (Utilities|FlowControl|Delay 0.2)
  (CallFunction|CheckCombinedElement))

(event Custom|ClearManagerSequence
  (Variables|Default|SetToolUsed "")
  (Variables|Default|SetElementUsed ""))

(event Custom|CheckCombinedElement
  (bind _toolused (Variables|Default|GetToolUsed))
  (bind _elementused (Variables|Default|GetElementUsed))
  (bind (_name _visualimage _direction1 _direction2 _direction3) (Utilities|Struct|BreakS_Séquence _toolused))
  (bind (_name_2 _visualimage_2 _direction1_2 _direction2_2 _direction3_2) (Utilities|Struct|BreakS_Séquence _elementused))
  (for _array_element (Variables|Default|GetResultList)
    (if (Math|Boolean|ANDBoolean (Utilities|Enum|Equal(Enum) (.Direction1 (Utilities|Struct|BreakS_Result _array_element)) _direction1_2) (Utilities|Enum|Equal(Enum) _direction2_2 (.Direction2 (Utilities|Struct|BreakS_Result _array_element))) (Utilities|Enum|Equal(Enum) (.Direction3 (Utilities|Struct|BreakS_Result _array_element)) _direction3_2) (Utilities|Enum|Equal(Enum) (.Direction4 (Utilities|Struct|BreakS_Result _array_element)) _direction1) (Utilities|Enum|Equal(Enum) (.Direction5 (Utilities|Struct|BreakS_Result _array_element)) _direction2) (Utilities|Enum|Equal(Enum) (.Direction6 (Utilities|Struct|BreakS_Result _array_element)) _direction3))
      (bind _output_get (Variables|Default|SetResult _array_element))
      (Development|PrintString (.Name (Utilities|Struct|BreakS_Result _output_get)))
      (Default|DeliveryDone (Variables|/Game/WSFGSProduction/UI/WBPUI_Game.WBPUI_Game_C|GetUI_QuestRequest (Variables|/Game/WSFGSProduction/Player/BP_Character.BP_Character_C|GetUi (Variables|Default|GetPlayer))) _output_get)
      (Audio|PlaySound2D "/Game/WSFGSProduction/Import/sound/CreatObject.CreatObject" 1.0 1.0 0.0 0 0))))

(event Custom|UnlockStone
  (Utilities|FlowControl|DoOnce false
    (:Completed
      (Default|CreateTag (Variables|/Game/WSFGSProduction/Player/BP_Character.BP_Character_C|GetUi (Variables|Default|GetPlayer)) (Utilities|Array|Get(acopy) (Variables|Default|GetListElement))))))

(event EventBeginPlay
  (CallFunction|CreateDelivery 2))

(fn ConstructionScript)