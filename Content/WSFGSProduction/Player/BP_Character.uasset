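; Player character that reads three-direction input combos (up, down, left, right) and matches them against a list of named sequences.
; Each press appends to the current attempt, updates the UI_Game widget created at BeginPlay, then prunes non-matching entries from a working candidate list.
; A single survivor at the third input validates; an empty list shows an error and blocks input for a second before resetting.
; Debug prints trace attempts and candidates, and a debug key clears the attempt.
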(event Custom|ResetSequence
  (Variables|Condition|SetCanUse false)
  (Default|CrossWrong (Variables|Default|GetUi))
  ;[0.15 0.15 0.15 0.5] Feedback erreur + delay
  (Utilities|FlowControl|Delay 1.0)
  (Variables|Condition|SetCanUse true)
  ;[0.15 0.15 0.15 0.5] Reset séquence joueur
  (Utilities|Array|Clear (Variables|Sequence|GetSequenceActual))
  ;[0.15 0.15 0.15 0.5] Reset sequence Check
  (Variables|Sequence|SetSéquenceCheck (Variables|Sequence|GetSéquenceAll))
  ;[0.15 0.15 0.15 0.5] Ajouter update sur UI
  (Default|ClearSequecneActuel (Variables|Default|GetUi)))

(event Custom|ValidateSequence
  (params (SéquenceValidated :type S%20Séquence%20Structure))
  (Default|OnSucess (Variables|Default|GetUi))
  (Development|PrintString (Utilities|String|ToString(Text) (.Name (Utilities|Struct|BreakS_Séquence SéquenceValidated))) true true "(R=1.000000,G=0.911978,B=0.150344,A=1.000000)")
  (Variables|Condition|SetCanUse true)
  ;[0.15 0.15 0.15 0.5] Reset séquence joueur
  (Utilities|Array|Clear (Variables|Sequence|GetSequenceActual))
  ;[0.15 0.15 0.15 0.5] Reset sequence Check
  (Variables|Sequence|SetSéquenceCheck (Variables|Sequence|GetSéquenceAll))
  ;[0.15 0.15 0.15 0.5] Ajouter update sur UI
  (Default|ClearSequecneActuel (Variables|Default|GetUi)))

(event Input|EnhancedActionEvents|EnhancedInputActionAI_Down
  (params (ActionValue :type Boolean) (ElapsedSeconds :type Float%20%28double-precision%29) (TriggeredSeconds :type Float%20%28double-precision%29) (InputAction :type Input%20Action%20Object%20Reference :default "/Game/WSFGSProduction/Controls/Input/AI_Down.AI_Down"))
  (bind _séquencecheck (Variables|Sequence|GetSéquenceCheck))
  (bind _returnvalue (Utilities|Array|Length _séquencecheck))
  ;[0.03427 0.15 0.04934 0.5] Entre une direction
  (:Started
    (if (Variables|Condition|GetCanUse)
      (Development|PrintString "down")
      ;[0.03427 0.15 0.04934 0.5] Ajoute la direction à l'array de tentative actuel
      (Utilities|Array|Add (Variables|Sequence|GetSequenceActual) "NewEnumerator1")
      (Default|Pressed (Variables|Default|GetUi) "NewEnumerator1")
      ;[0.15 0.03734 0.04307 0.5] Compare l'élément à celui de la suite actuel (si le nouvel élément est pas égale a celui dans la séquence on retire la sequence de la liste) si la liste atteind 1 ou 0 on finit)
      (Default|ReceiveSequenceActual (Variables|Default|GetUi) (Variables|Sequence|GetSequenceActual))
      (Utilities|FlowControl|Sequence
        (:then_0
          (|DebugActualSequence))
        (:then_1
          (for (_array_element _array_index) (Variables|Sequence|GetSequenceActual)
            (if (== _array_index 0)
              ;;[0.15 0.132 0.132 0.5] Retirer les éléments qui n'on pas la même suite de la liste
              (for _array_element_2 (Variables|Sequence|GetSéquenceAll)
                (if (not (Utilities|Enum|Equal(Enum) _array_element (.Direction1 (Utilities|Struct|BreakS_Séquence _array_element_2))))
                  (Utilities|Array|RemoveItem (Variables|Sequence|GetSéquenceCheck) _array_element_2)
                  ;;[0.15 0.1364 0.1349 0.5] Si aucun élément faire echec
                  (if (<= (Utilities|Array|Length (Variables|Sequence|GetSéquenceCheck)) 0)
                    (CallFunction|ResetSequence))))
              (elif (== _array_index 1)
                (for _array_element_3 (Variables|Sequence|GetSéquenceAll)
                  (if (not (Utilities|Enum|Equal(Enum) _array_element (.Direction2 (Utilities|Struct|BreakS_Séquence _array_element_3))))
                    (Utilities|Array|RemoveItem (Variables|Sequence|GetSéquenceCheck) _array_element_3)
                    (if (<= (Utilities|Array|Length (Variables|Sequence|GetSéquenceCheck)) 0)
                      (CallFunction|ResetSequence))))
                (elif (== _array_index 2)
                  (for _array_element_4 (Variables|Sequence|GetSéquenceAll)
                    (if (Utilities|Enum|Equal(Enum) _array_element (.Direction3 (Utilities|Struct|BreakS_Séquence _array_element_4)))
                      (Utilities|FlowControl|Delay 0.05)
                      ;;[0.15 0.1408 0.1394 0.5] Si élément correspon exactement faire quelque chose
                      (if (== _returnvalue 1)
                        (bind _output_get (Variables|Sequence|SetSéquenceActivé (Utilities|Array|Get(acopy) (Variables|Sequence|GetSéquenceCheck))))
                        (CallFunction|ValidateSequence _output_get)
                        (elif (== _returnvalue 0)
                          (CallFunction|ResetSequence)))
                      (else
                        (Utilities|Array|RemoveItem (Variables|Sequence|GetSéquenceCheck) _array_element_4))))))))
          (|DébugFeedbackListOfElement)))))
  (:Completed
    (Default|Release (Variables|Default|GetUi))))

(event Input|EnhancedActionEvents|EnhancedInputActionAI_Left
  (params (ActionValue :type Boolean) (ElapsedSeconds :type Float%20%28double-precision%29) (TriggeredSeconds :type Float%20%28double-precision%29) (InputAction :type Input%20Action%20Object%20Reference :default "/Game/WSFGSProduction/Controls/Input/AI_Left.AI_Left"))
  (bind _séquencecheck (Variables|Sequence|GetSéquenceCheck))
  (bind _returnvalue (Utilities|Array|Length _séquencecheck))
  ;[0.03427 0.15 0.04934 0.5] Entre une direction
  (:Started
    (if (Variables|Condition|GetCanUse)
      (Development|PrintString "left")
      ;[0.03427 0.15 0.04934 0.5] Ajoute la direction à l'array de tentative actuel
      (Utilities|Array|Add (Variables|Sequence|GetSequenceActual) "NewEnumerator2")
      (Default|Pressed (Variables|Default|GetUi) "NewEnumerator2")
      ;[0.15 0.03734 0.04307 0.5] Compare l'élément à celui de la suite actuel (si le nouvel élément est pas égale a celui dans la séquence on retire la sequence de la liste) si la liste atteind 1 ou 0 on finit)
      (Default|ReceiveSequenceActual (Variables|Default|GetUi) (Variables|Sequence|GetSequenceActual))
      (Utilities|FlowControl|Sequence
        (:then_0
          (|DebugActualSequence))
        (:then_1
          (for (_array_element _array_index) (Variables|Sequence|GetSequenceActual)
            (if (== _array_index 0)
              ;;[0.15 0.132 0.132 0.5] Retirer les éléments qui n'on pas la même suite de la liste
              (for _array_element_2 (Variables|Sequence|GetSéquenceAll)
                (if (not (Utilities|Enum|Equal(Enum) _array_element (.Direction1 (Utilities|Struct|BreakS_Séquence _array_element_2))))
                  (Utilities|Array|RemoveItem (Variables|Sequence|GetSéquenceCheck) _array_element_2)
                  ;;[0.15 0.1364 0.1349 0.5] Si aucun élément faire echec
                  (if (<= (Utilities|Array|Length (Variables|Sequence|GetSéquenceCheck)) 0)
                    (CallFunction|ResetSequence))))
              (elif (== _array_index 1)
                (for _array_element_3 (Variables|Sequence|GetSéquenceAll)
                  (if (not (Utilities|Enum|Equal(Enum) _array_element (.Direction2 (Utilities|Struct|BreakS_Séquence _array_element_3))))
                    (Utilities|Array|RemoveItem (Variables|Sequence|GetSéquenceCheck) _array_element_3)
                    (if (<= (Utilities|Array|Length (Variables|Sequence|GetSéquenceCheck)) 0)
                      (CallFunction|ResetSequence))))
                (elif (== _array_index 2)
                  (for _array_element_4 (Variables|Sequence|GetSéquenceAll)
                    (if (Utilities|Enum|Equal(Enum) _array_element (.Direction3 (Utilities|Struct|BreakS_Séquence _array_element_4)))
                      (Utilities|FlowControl|Delay 0.05)
                      ;;[0.15 0.1408 0.1394 0.5] Si élément correspon exactement faire quelque chose
                      (if (== _returnvalue 1)
                        (bind _output_get (Variables|Sequence|SetSéquenceActivé (Utilities|Array|Get(acopy) (Variables|Sequence|GetSéquenceCheck))))
                        (CallFunction|ValidateSequence _output_get)
                        (elif (== _returnvalue 0)
                          (CallFunction|ResetSequence)))
                      (else
                        (Utilities|Array|RemoveItem (Variables|Sequence|GetSéquenceCheck) _array_element_4))))))))
          (|DébugFeedbackListOfElement)))))
  (:Completed
    (Default|Release (Variables|Default|GetUi))))

(event Input|EnhancedActionEvents|EnhancedInputActionAI_Right
  (params (ActionValue :type Boolean) (ElapsedSeconds :type Float%20%28double-precision%29) (TriggeredSeconds :type Float%20%28double-precision%29) (InputAction :type Input%20Action%20Object%20Reference :default "/Game/WSFGSProduction/Controls/Input/AI_Right.AI_Right"))
  (bind _séquencecheck (Variables|Sequence|GetSéquenceCheck))
  (bind _returnvalue (Utilities|Array|Length _séquencecheck))
  ;[0.03427 0.15 0.04934 0.5] Entre une direction
  (:Started
    (if (Variables|Condition|GetCanUse)
      (Development|PrintString "right")
      ;[0.03427 0.15 0.04934 0.5] Ajoute la direction à l'array de tentative actuel
      (Utilities|Array|Add (Variables|Sequence|GetSequenceActual) "NewEnumerator3")
      (Default|Pressed (Variables|Default|GetUi) "NewEnumerator3")
      ;[0.15 0.03734 0.04307 0.5] Compare l'élément à celui de la suite actuel (si le nouvel élément est pas égale a celui dans la séquence on retire la sequence de la liste) si la liste atteind 1 ou 0 on finit)
      (Default|ReceiveSequenceActual (Variables|Default|GetUi) (Variables|Sequence|GetSequenceActual))
      (Utilities|FlowControl|Sequence
        (:then_0
          (|DebugActualSequence))
        (:then_1
          (for (_array_element _array_index) (Variables|Sequence|GetSequenceActual)
            (if (== _array_index 0)
              ;;[0.15 0.132 0.132 0.5] Retirer les éléments qui n'on pas la même suite de la liste
              (for _array_element_2 (Variables|Sequence|GetSéquenceAll)
                (if (not (Utilities|Enum|Equal(Enum) _array_element (.Direction1 (Utilities|Struct|BreakS_Séquence _array_element_2))))
                  (Utilities|Array|RemoveItem (Variables|Sequence|GetSéquenceCheck) _array_element_2)
                  ;;[0.15 0.1364 0.1349 0.5] Si aucun élément faire echec
                  (if (<= (Utilities|Array|Length (Variables|Sequence|GetSéquenceCheck)) 0)
                    (CallFunction|ResetSequence))))
              (elif (== _array_index 1)
                (for _array_element_3 (Variables|Sequence|GetSéquenceAll)
                  (if (not (Utilities|Enum|Equal(Enum) _array_element (.Direction2 (Utilities|Struct|BreakS_Séquence _array_element_3))))
                    (Utilities|Array|RemoveItem (Variables|Sequence|GetSéquenceCheck) _array_element_3)
                    (if (<= (Utilities|Array|Length (Variables|Sequence|GetSéquenceCheck)) 0)
                      (CallFunction|ResetSequence))))
                (elif (== _array_index 2)
                  (for _array_element_4 (Variables|Sequence|GetSéquenceAll)
                    (if (Utilities|Enum|Equal(Enum) _array_element (.Direction3 (Utilities|Struct|BreakS_Séquence _array_element_4)))
                      (Utilities|FlowControl|Delay 0.05)
                      ;;[0.15 0.1408 0.1394 0.5] Si élément correspon exactement faire quelque chose
                      (if (== _returnvalue 1)
                        (bind _output_get (Variables|Sequence|SetSéquenceActivé (Utilities|Array|Get(acopy) (Variables|Sequence|GetSéquenceCheck))))
                        (CallFunction|ValidateSequence _output_get)
                        (elif (== _returnvalue 0)
                          (CallFunction|ResetSequence)))
                      (else
                        (Utilities|Array|RemoveItem (Variables|Sequence|GetSéquenceCheck) _array_element_4))))))))
          (|DébugFeedbackListOfElement)))))
  (:Completed
    (Default|Release (Variables|Default|GetUi))))

(event Input|EnhancedActionEvents|EnhancedInputActionAI_Up
  (params (ActionValue :type Boolean) (ElapsedSeconds :type Float%20%28double-precision%29) (TriggeredSeconds :type Float%20%28double-precision%29) (InputAction :type Input%20Action%20Object%20Reference :default "/Game/WSFGSProduction/Controls/Input/AI_Up.AI_Up"))
  (bind _séquencecheck (Variables|Sequence|GetSéquenceCheck))
  (bind _returnvalue (Utilities|Array|Length _séquencecheck))
  ;[0.03427 0.15 0.04934 0.5] Entre une direction
  (:Started
    (if (Variables|Condition|GetCanUse)
      (Development|PrintString "up")
      ;[0.03427 0.15 0.04934 0.5] Ajoute la direction à l'array de tentative actuel
      (Utilities|Array|Add (Variables|Sequence|GetSequenceActual) "NewEnumerator0")
      (Default|Pressed (Variables|Default|GetUi) "NewEnumerator0")
      ;[0.15 0.03734 0.04307 0.5] Compare l'élément à celui de la suite actuel (si le nouvel élément est pas égale a celui dans la séquence on retire la sequence de la liste) si la liste atteind 1 ou 0 on finit)
      (Default|ReceiveSequenceActual (Variables|Default|GetUi) (Variables|Sequence|GetSequenceActual))
      (Utilities|FlowControl|Sequence
        (:then_0
          (|DebugActualSequence))
        (:then_1
          (for (_array_element _array_index) (Variables|Sequence|GetSequenceActual)
            (if (== _array_index 0)
              ;;[0.15 0.132 0.132 0.5] Retirer les éléments qui n'on pas la même suite de la liste
              (for _array_element_2 (Variables|Sequence|GetSéquenceAll)
                (if (not (Utilities|Enum|Equal(Enum) _array_element (.Direction1 (Utilities|Struct|BreakS_Séquence _array_element_2))))
                  (Utilities|Array|RemoveItem (Variables|Sequence|GetSéquenceCheck) _array_element_2)
                  ;;[0.15 0.1364 0.1349 0.5] Si aucun élément faire echec
                  (if (<= (Utilities|Array|Length (Variables|Sequence|GetSéquenceCheck)) 0)
                    (CallFunction|ResetSequence))))
              (elif (== _array_index 1)
                (for _array_element_3 (Variables|Sequence|GetSéquenceAll)
                  (if (not (Utilities|Enum|Equal(Enum) _array_element (.Direction2 (Utilities|Struct|BreakS_Séquence _array_element_3))))
                    (Utilities|Array|RemoveItem (Variables|Sequence|GetSéquenceCheck) _array_element_3)
                    (if (<= (Utilities|Array|Length (Variables|Sequence|GetSéquenceCheck)) 0)
                      (CallFunction|ResetSequence))))
                (elif (== _array_index 2)
                  (for _array_element_4 (Variables|Sequence|GetSéquenceAll)
                    (if (Utilities|Enum|Equal(Enum) _array_element (.Direction3 (Utilities|Struct|BreakS_Séquence _array_element_4)))
                      (Utilities|FlowControl|Delay 0.05)
                      ;;[0.15 0.1408 0.1394 0.5] Si élément correspon exactement faire quelque chose
                      (if (== _returnvalue 1)
                        (bind _output_get (Variables|Sequence|SetSéquenceActivé (Utilities|Array|Get(acopy) (Variables|Sequence|GetSéquenceCheck))))
                        (CallFunction|ValidateSequence _output_get)
                        (elif (== _returnvalue 0)
                          (CallFunction|ResetSequence)))
                      (else
                        (Utilities|Array|RemoveItem (Variables|Sequence|GetSéquenceCheck) _array_element_4))))))))
          (|DébugFeedbackListOfElement)))))
  (:Completed
    (Default|Release (Variables|Default|GetUi))))

(event Input|EnhancedActionEvents|EnhancedInputActionAI_DebugSpaceBar
  (params (ActionValue :type Boolean) (ElapsedSeconds :type Float%20%28double-precision%29) (TriggeredSeconds :type Float%20%28double-precision%29) (InputAction :type Input%20Action%20Object%20Reference :default "/Game/WSFGSProduction/Controls/Input/AI_DebugSpaceBar.AI_DebugSpaceBar"))
  (:Started
    ;[0.15 0.15 0.15 0.5] Reset séquence joueur
    (Utilities|Array|Clear (Variables|Sequence|GetSequenceActual))
    ;[0.15 0.15 0.15 0.5] Reset sequence Check
    (Variables|Sequence|SetSéquenceCheck (Variables|Sequence|GetSéquenceAll))
    ;[0.15 0.15 0.15 0.5] Ajouter update sur UI
    (Default|ClearSequecneActuel (Variables|Default|GetUi))))

(event EventBeginPlay
  (Variables|Sequence|SetSéquenceCheck (Variables|Sequence|GetSéquenceAll))
  (Variables|/Script/Engine.PlayerController|SetbShowMouseCursor (Game|GetPlayerController 0) true)
  (bind _returnvalue (UserInterface|CreateWidget "/Game/WSFGSProduction/UI/UI_Game.UI_Game_C" (Game|GetPlayerController 0)))
  (bind _output_get (Variables|Default|SetUi _returnvalue))
  (UserInterface|Viewport|AddtoViewport _output_get 0))

(fn ConstructionScript)